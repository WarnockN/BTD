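; BP_Payload is a payload Blueprint that tracks an integer Health value, with functions to raise or lower it in fixed steps.
; Increase and decrease check that the current Health is in range, call AdjustHealthBar with the new value, then store it.
; AdjustHealthBar only prints a negated, offset float of that value; no health bar is updated.
; The range check precedes the change, so Health can step past its bounds.
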(fn `Adjust Health Bar`
  (params (Health :type Integer))
  (`KismetSystemLibrary.PrintString` (`KismetStringLibrary.Conv_DoubleToString` (+ (`KismetMathLibrary.Conv_IntToDouble` (* Health -1)) 1.0))))

(fn `DecreaseHealthBar`
  (bind _returnvalue (- (`self.Health`) 10))
  (if (`KismetMathLibrary.InRange_IntInt` (`self.Health`) 0 100)
    (`self.Adjust Health Bar` _returnvalue)
    (set `self.Health` _returnvalue)))

(fn `IncreaseHealthBar`
  (bind _returnvalue (+ (`self.Health`) 10))
  (if (`KismetMathLibrary.InRange_IntInt` (`self.Health`) 0 100)
    (`self.Adjust Health Bar` _returnvalue)
    (set `self.Health` _returnvalue)))

(fn `UserConstructionScript`)