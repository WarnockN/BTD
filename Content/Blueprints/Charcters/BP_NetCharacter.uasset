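; BP_NetCharacter is a character Blueprint that sets up the on-screen HUD for the locally controlled player.
; On BeginPlay, if locally controlled, it creates the WB_Crosshair and WB_Health widgets and adds both to the viewport.
; On Tick, the same local-control check gates a debug print of the current Health from HealthComp.
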(event `self.ReceiveBeginPlay`
  (if (`self.IsLocallyControlled`)
    (`|ExecutionSequence`
      (:`then_0`
        (bind _returnvalue (`|CreateWidget` "/Game/UI/WB_Crosshair.WB_Crosshair_C"))
        (`UserWidget.AddToViewport` _returnvalue 0))
      (:`then_1`
        (bind _returnvalue_2 (`|CreateWidget` "/Game/UI/WB_Health.WB_Health_C"))
        (`UserWidget.AddToViewport` _returnvalue_2 0)))))

(event `self.ReceiveTick`
  (params (DeltaSeconds :type "Float (single-precision)"))
  (if (`self.IsLocallyControlled`)
    (`KismetSystemLibrary.PrintString` (`KismetStringLibrary.Conv_DoubleToString` (`HealthComponent.Health` (`self.HealthComp`))) true true (struct :`R` 1.0 :`G` 0.887439 :`A` 1.0) 0.0)))

(fn `UserConstructionScript`)