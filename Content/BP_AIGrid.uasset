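; BP_AIGrid is an actor that previews an AI grid with debug drawing; its event graph contains no logic.
; The construction script flushes persistent debug lines, then draws the grid's boundary box around the scene component's location.
; It marks the corner returned by GridBottomLeft, calls DrawTile, and draws a tile-sized plane at TilePosition, slightly shrunk by a fixed margin.
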(event `self.ReceiveBeginPlay`)

(event `self.ReceiveTick`
  (params (DeltaSeconds :type "Float (single-precision)")))

(fn `UserConstructionScript`
  (bind (_gridsizeworld_x _gridsizeworld_y) (`KismetMathLibrary.BreakVector2D` (`self.GridSizeWorld`)))
  (`KismetSystemLibrary.FlushPersistentDebugLines`)
  (bind _output_get (set `self.GridLocation` (`SceneComponent.K2_GetComponentLocation` (`self.Scene1`))))
  (`KismetSystemLibrary.DrawDebugBox` _output_get (`KismetMathLibrary.MakeVector` _gridsizeworld_x _gridsizeworld_y 5.0) (`self.GridColor`) (struct) 1000.0 10.0)
  (bind _returnvalue (`self.GridBottomLeft`))
  (`KismetSystemLibrary.DrawDebugBox` _returnvalue (20.0 20.0 20.0) (struct :`R` 0.034115 :`G` 1.0 :`A` 1.0) (struct) 1000.0 10.0)
  (`self.DrawTile`)
  (`KismetSystemLibrary.DrawDebugPlane` (make `Plane` 0.0 0.0 0.0 1.0) (`self.TilePosition`) (- (`self.TileSize`) 5.0) (struct :`R` 0.969393 :`G` 1.0 :`A` 1.0) 100.0))